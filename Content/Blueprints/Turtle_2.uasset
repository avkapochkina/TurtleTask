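; Turtle actor that moves in a stop-and-go rhythm.
; BeginPlay caches the starting Speed and starts a looping half-second timer that toggles Speed between zero and that cached value.
; Tick calls Movement, which is not defined in this graph, every frame.
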(event `self.ReceiveBeginPlay`
  (set `self.DefaultSpeed` (`self.Speed`))
  (`KismetSystemLibrary.K2_SetTimerDelegate` (delegate `SetNewSpeed`) 0.5 true))

(event `SetNewSpeed`
  (if (== (`self.Speed`) (`self.DefaultSpeed`))
    (set `self.Speed` 0.0)
    (else
      (set `self.Speed` (`self.DefaultSpeed`)))))

(event `self.ReceiveTick`
  (params (DeltaSeconds :type "Float (single-precision)"))
  (`self.Movement`))

(fn `UserConstructionScript`)